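; BP_Boss is a boss character with a montage-driven melee attack, its own health bar widget and ragdoll death.
; Attack plays a montage guarded against re-entry, whose notify sphere-traces between two components to damage a hit pawn and plays a world camera shake.
; Incoming damage lowers Health, which Tick pushes to the widget, and at zero movement stops and the mesh simulates physics.
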(event EventAttack
  ;[1 1 1] Attack
  (if (not (Variables|Default|GetisAttacking))
    (Animation|Montage|PlayMontage (Variables|Character|GetMesh) "/Game/Ancient_Golem/Demo/ThirdPersonJump_Start_Montage.ThirdPersonJump_Start_Montage"
      (:then
        (Variables|Default|SetisAttacking true))
      (:OnCompleted
        (Variables|Default|SetisAttacking false))
      (:OnNotifyBegin
        (Utilities|FlowControl|Sequence
          (:then_0
            (bind (_outhit _returnvalue) (Collision|SphereTraceForObjects (Transformation|GetSocketLocation (Variables|Default|GetStartAttack%20) "None") (Transformation|GetSocketLocation (Variables|Default|GetEndAttack) "None") 8e+01 (Utilities|Array|MakeArray "ObjectTypeQuery3") false 0 "ForDuration" true "(R=1.000000,G=0.000000,B=0.000000,A=1.000000)" "(R=0.000000,G=1.000000,B=0.000000,A=1.000000)" 2.0))
            (if _returnvalue
              (Game|Damage|ApplyDamage (.HitActor (Collision|BreakHitResult _outhit)) 2.0 0 0)))
          (:then_1
            (Camera|PlayWorldCameraShake "/Game/Assets/Boss/BP_Attack_CameraShake.BP_Attack_CameraShake_C" (Transformation|GetActorLocation) 0.0 3.5e+03)))))))

(event EventBeginPlay
  (bind _returnvalue (UserInterface|CreateWidget "/Game/Assets/Boss/WB_BossHealth.WB_BossHealth_C"))
  (UserInterface|Viewport|AddtoViewport _returnvalue 0)
  (Variables|Default|Sethealth%20UI _returnvalue))

(event EventTick
  (params (DeltaSeconds :type Float%20%28single-precision%29))
  (Progress|SetPercent (Variables|/Game/Assets/Boss/WB_BossHealth.WB_BossHealth_C|GetHealthBar (Variables|Default|Gethealth%20UI)) (/ (Variables|Default|Gethealth) 1e+03)))

(event Game|Damage|EventAnyDamage
  (params (Damage :type Float%20%28single-precision%29) (DamageType :type Damage%20Type%20Object%20Reference) (InstigatedBy :type Controller%20Object%20Reference) (DamageCauser :type Actor%20Object%20Reference))
  (Variables|Default|Sethealth (- (Variables|Default|Gethealth) Damage))
  (if (<= (Variables|Default|Gethealth) 0.0)
    (Pawn|Components|CharacterMovement|DisableMovement (Variables|Character|GetCharacterMovement))
    (Physics|SetSimulatePhysics (Variables|Character|GetMesh) true)))

(fn ConstructionScript)
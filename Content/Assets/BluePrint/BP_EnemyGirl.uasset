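; Enemy girl AI character that patrols a path of placed actors and chases the player on sight.
; Patrol walks to each EnemyPath point via AIMoveTo, pauses, then advances the looping index.
; PawnSensing sets ISeePlayer and starts a faster chase, which returns to patrol only after reaching the player.
; The two events call each other without a behavior tree, and failed moves are not handled.
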(event OnSeePawn(PawnSensing)
  (params (Pawn :type Pawn%20Object%20Reference))
  (Variables|Default|SetISeePlayer true)
  (CallFunction|FollowPlayer))

(event Custom|FollowPlayer
  ;[1 1 1] Follow Player
  (if (Variables|Default|GetISeePlayer)
    (Variables|/Script/Engine.CharacterMovementComponent|SetMaxWalkSpeed (Variables|Character|GetCharacterMovement) 5e+02)
    (AI|AIMoveTo self "0, 0, 0" (Game|GetPlayerCharacter 0) 1e+01 false
      (:OnSuccess
        (Variables|Default|SetISeePlayer false)
        (CallFunction|EnemyPatrol)))
    (else
      (Variables|Default|SetISeePlayer false)
      (CallFunction|EnemyPatrol))))

(event Custom|EnemyPatrol
  (bind _enemypath (Variables|Default|GetEnemyPath))
  ;[1 1 1] Enemy Patrol
  (if (Variables|Default|GetISeePlayer)
    (CallFunction|FollowPlayer)
    (else
      (Variables|/Script/Engine.CharacterMovementComponent|SetMaxWalkSpeed (Variables|Character|GetCharacterMovement) 3e+02)
      (AI|AIMoveTo self (Transformation|GetActorLocation (Utilities|Array|Get(acopy) _enemypath (Variables|Default|GetIndex))) 0 5.0 false
        (:OnSuccess
          (Utilities|FlowControl|Delay 3.0)
          (if (>= (Variables|Default|GetIndex) (- (Utilities|Array|Length _enemypath) 1))
            (Variables|Default|SetIndex 0)
            (else
              (Math|Integer|IncrementInt (Variables|Default|GetIndex)
                (:%20%20
                  _))))
          (CallFunction|EnemyPatrol))))))

(event EventBeginPlay
  (CallFunction|EnemyPatrol))

(event Collision|EventActorBeginOverlap
  (params (OtherActor :type Actor%20Object%20Reference)))

(event EventTick
  (params (DeltaSeconds :type Float%20%28single-precision%29)))

(fn ConstructionScript)
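; Melee enemy that chases the player on sight, attacks up close, and has an even chance to spawn a BP_Life when killed.
; PawnSensing sets a sight flag that is never cleared and triggers AIMoveTo toward the player.
; On arrival it alternates two boxing animations, damages Player-tagged actors via sphere overlap, then restores the AnimBP after a cooldown.
; Tick halts movement until the player is seen and turns the widget toward the camera.
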(event OnSeePawn(PawnSensing)
  (params (Pawn :type Pawn%20Object%20Reference))
  (Variables|Default|SetiSeePlayer true)
  (CallFunction|FollowPlayer))

(event Custom|FollowPlayer
  (if (Variables|Default|GetiSeePlayer)
    (AI|AIMoveTo self "0, 0, 0" (Game|GetPlayerCharacter 0) 1e+01 false
      (:OnSuccess
        (if (Variables|Default|GetcanAttack)
          (Variables|Default|SetcanAttack false)
          (CallFunction|RandomAnim)
          (bind _outactors (Collision|SphereOverlapActors (Transformation|GetWorldLocation (Variables|Default|GetArrow1)) 1e+02 (Variables|Default|GetObject%20Types) 0))
          (bind _array_element (Utilities|Array|ForEachLoopwithBreak _outactors)
            (:LoopBody
              (if (Actor|ActorHasTag _array_element "Player")
                (Game|Damage|ApplyDamage _array_element 5.0 0 0)))
            (:Completed
              (Utilities|FlowControl|Delay 1.1)
              (Class|SkeletalMeshComponent|SetAnimClass (Variables|Character|GetMesh) "/Game/Assets/Animation/Enemy/BPA_Enemy1.BPA_Enemy1_C")
              (Variables|Default|SetcanAttack true))))))))

(event Custom|RandomAnim
  (if (== (Variables|Default|GetattackNum) 0)
    (Components|Animation|PlayAnimation (Variables|Character|GetMesh) "/Game/Assets/Animation/Enemy/Boxing.Boxing" false)
    (Variables|Default|SetattackNum 1)
    (else
      (Components|Animation|PlayAnimation (Variables|Character|GetMesh) "/Game/Assets/Animation/Enemy/Boxing_2.Boxing_2" false)
      (Variables|Default|SetattackNum 0))))

(event Custom|SpawnLife
  (Variables|Default|SetnumRandoms (Math|Random|RandomIntegerinRange 0 1))
  (if (== (Variables|Default|GetnumRandoms) 0)
    (Game|SpawnActorfromClass "/Game/Assets/BluePrint/BP_Life.BP_Life_C" (Transformation|GetActorTransform) "Undefined" "MultiplyWithRoot" 0 0)))

(event EventTick
  (params (DeltaSeconds :type Float%20%28single-precision%29))
  (Utilities|FlowControl|Sequence
    (:then_0
      (if (not (Variables|Default|GetiSeePlayer))
        (Components|Movement|StopMovementImmediately (Variables|Character|GetCharacterMovement))))
    (:then_1
      (Transformation|SetWorldRotation (Variables|Default|GetWidget) (Math|Rotator|FindLookatRotation (Transformation|GetWorldLocation (Variables|Default|GetWidget)) (Transformation|GetWorldLocation (Variables|/Script/Engine.PlayerCameraManager|GetTransformComponent (Game|GetPlayerCameraManager 0)))) false false))))

(event Game|Damage|EventAnyDamage
  (params (Damage :type Float%20%28single-precision%29) (DamageType :type Damage%20Type%20Object%20Reference) (InstigatedBy :type Controller%20Object%20Reference) (DamageCauser :type Actor%20Object%20Reference))
  (Variables|Default|Sethealth (- (Variables|Default|Gethealth) Damage))
  (Development|PrintString (Utilities|String|ToString(Float) (Variables|Default|Gethealth)))
  (if (<= (Variables|Default|Gethealth) 0.0)
    (Actor|DestroyActor)
    (CallFunction|SpawnLife)))

(fn ConstructionScript)
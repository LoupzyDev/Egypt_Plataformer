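; Player scan ability that fires an expanding pulse with sound and post-process effects, revealing nearby objects.
; StartScan is gated by a DoOnce that Tick resets after a cooldown, and writes the player position to MPC_Controller for the materials.
; A timeline drives both the material radius and a growing sphere trace that sends EnableTargetMessage to hit actors.
; A second timeline fades the after-scan blend in and out around the pulse.
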(event Custom|AfterScanEffect
  (params (reverse? :type Boolean))
  ;[1 1 1] Fade Effect
  (if reverse?
    (bind _newtrack_0 (Timeline|ToGreyTL ReverseFromEnd)
      (:Update
        (Variables|/Script/Engine.PostProcessComponent|SetBlendWeight (Variables|Default|GetAfterPostProcess) _newtrack_0)
        (Rendering|Material|SetScalarParameterValue "/Game/ScanFX/Materials/MPC/MPC_Controller.MPC_Controller" "Alpha" _newtrack_0 :!class /Script/Engine.KismetMaterialLibrary)))
    (else
      (Timeline|ToGreyTL PlayFromStart))))

(event Custom|StartScan
  (bind _returnvalue (Transformation|GetActorLocation))
  (bind _returnvalue_2 (Transformation|GetActorLocation))
  ;[1 1 1] Scan Implemantation
  (Utilities|FlowControl|DoOnce false
    (:Completed
      (Utilities|FlowControl|Sequence
        (:then_0
          (Variables|Settings|SetScanModeActive? true)
          (Variables|Settings|SetElapsedTime 0.0))
        (:then_1
          (Rendering|Material|SetScalarParameterValue "/Game/ScanFX/Materials/MPC/MPC_Controller.MPC_Controller" "PlayerX" (.x _returnvalue) :!class /Script/Engine.KismetMaterialLibrary)
          (Rendering|Material|SetScalarParameterValue "/Game/ScanFX/Materials/MPC/MPC_Controller.MPC_Controller" "PlayerY" (.y _returnvalue) :!class /Script/Engine.KismetMaterialLibrary)
          (Rendering|Material|SetScalarParameterValue "/Game/ScanFX/Materials/MPC/MPC_Controller.MPC_Controller" "PlayerZ" (.z _returnvalue) :!class /Script/Engine.KismetMaterialLibrary))
        (:then_2
          (CallFunction|AfterScanEffect false)
          (CallFunction|PlaySFX)
          (bind _newtrack_0 (Timeline|ScanTimeLine PlayFromStart)
            (:Update
              (Rendering|Material|SetScalarParameterValue "/Game/ScanFX/Materials/MPC/MPC_Controller.MPC_Controller" "Radius" _newtrack_0 :!class /Script/Engine.KismetMaterialLibrary)
              ;;[1 1 1] Find Nearest Objects
              (bind (_outhits _returnvalue_3) (Collision|MultiSphereTraceForObjects _returnvalue_2 (+ _returnvalue_2 "0, 0,1.000000") (* _newtrack_0 5e+03) (Utilities|Array|MakeArray "ObjectTypeQuery2" "ObjectTypeQuery3") false 0 "None"))
              (if _returnvalue_3
                (for _array_element _outhits
                  (Class|BPITargetInterface|EnableTarget(Message) (.HitActor (Collision|BreakHitResult _array_element)) (Variables|Settings|GetDiscoveryDuration) (Transformation|GetActorLocation)))))
            (:Finished
              (CallFunction|AfterScanEffect true)
              (Utilities|FlowControl|Delay (Variables|Settings|GetDiscoveryDuration))
              (Rendering|Material|SetScalarParameterValue "/Game/ScanFX/Materials/MPC/MPC_Controller.MPC_Controller" "Radius" 0.0 :!class /Script/Engine.KismetMaterialLibrary))))))))

(event Custom|EnableScan
  (bind _returnvalue (Transformation|GetActorLocation))
  (bind _returnvalue_2 (Transformation|GetActorLocation))
  ;[1 1 1] Scan Implemantation
  (Utilities|FlowControl|DoOnce false) ; enters at Reset
)

(event Custom|PlaySFX
  ;[1 1 1] Scan SFX
  (Audio|PlaySoundatLocation (Variables|Settings|GetScanSFX) (Transformation|GetActorLocation) "0, 0, 0" 1.0 1.0 0.3 0 0 0 0))

(event EventBeginPlay)

(event EventTick
  (params (DeltaSeconds :type Float%20%28single-precision%29))
  ;[1 1 1] Event Tick
  (if (Variables|Settings|GetScanModeActive?)
    (bind _output_get (Variables|Settings|SetElapsedTime (+ DeltaSeconds (Variables|Settings|GetElapsedTime))))
    (if (>= _output_get (+ (Variables|Settings|GetScanDelay) 1.8))
      (CallFunction|EnableScan)
      (Variables|Settings|SetScanModeActive? false))))

(fn ConstructionScript
  (CallFunction|UpdatePostProcess)
  (Variables|Settings|SetElapsedTime (Variables|Settings|GetScanDelay)))

(fn UpdatePostProcess
  (Utilities|Struct|SetmembersinPostProcessSettings (Variables|/Script/Engine.PostProcessComponent|GetSettings (Variables|Default|GetAfterPostProcess)) (Utilities|Struct|MakeWeightedBlendables (Utilities|Array|MakeArray (Utilities|Struct|MakeWeightedBlendable 1.0 (Variables|Settings|GetAfter_ScanMaterial)))))
  (Utilities|Struct|SetmembersinPostProcessSettings (Variables|/Script/Engine.PostProcessComponent|GetSettings (Variables|Default|GetScanPostProcess)) (Utilities|Struct|MakeWeightedBlendables (Utilities|Array|MakeArray (Utilities|Struct|MakeWeightedBlendable 1.0 (Variables|Settings|GetScanMaterial))))))
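; BP_Target_Actor is a scannable target that is temporarily highlighted and shows a HUD marker when discovered.
; On BeginPlay it caches the WBP_Target from its widget component.
; DiscoverTarget enables custom depth on the supplied mesh and passes the rounded player distance in meters, timeout and display flags to the widget.
; A DoOnce blocks retriggering until the timeout delay ends and custom depth is turned off.
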(event Custom|Discover%20Target
  (params (Timeout :type Float%20%28double-precision%29) (Mesh :type Mesh%20Component%20Object%20Reference) (PlayerLocation :type Vector))
  ;[1 1 1] Main Functions to Implements
  (Utilities|FlowControl|DoOnce false :!label _label
    (:Completed
      (Rendering|SetRenderCustomDepth Mesh true)
      (Rendering|SetCustomDepthStencilValue Mesh 0)
      (Default|EnableHUD (Variables|Default|GetWdg%20Traget%20) (Math|Conversions|ToFloat(Integer) (Math|Float|Round (/ (Math|Vector|Distance(Vector) PlayerLocation (Transformation|GetWorldLocation Mesh)) 1e+02))) Timeout (Variables|Settings|GetDistance%20Enable?) (Variables|Settings|GetIcon%20Enable?))
      (Utilities|FlowControl|Delay Timeout)
      (Rendering|SetRenderCustomDepth Mesh false)
      (goto _label Reset))))

(event EventBeginPlay
  ;[1 1 1] Init Widget
  (bind _aswbp_target (Utilities|Casting|CastToWBP_Target (UserInterface|GetWidget (Variables|Default|GetWidget))))
  (Variables|Default|SetWdg%20Traget%20 _aswbp_target))

(fn ConstructionScript)
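; Demo target actor Blueprint for ScanFX, with a Cube mesh that can be revealed by a scan.
; On BeginPlay it casts its TargetActor child actor to BP_Target_Actor and caches the reference.
; EnableTarget forwards a timeout, the Cube and the player location to that actor's DiscoverTarget.
; A Rotate timeline that would spin the Cube through a full yaw turn exists but is never triggered.
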(event EventBeginPlay
  ;[1 1 1] Implemantaion Guide
  ;;[1 1 1] 3. Add This Functions inside BP
  (bind _asbp_target_actor (Utilities|Casting|CastToBP_Target_Actor (Variables|/Script/Engine.ChildActorComponent|GetChildActor (Variables|Default|GetTarget_Actor))))
  (Variables|Default|SetBP%20Target%20Actor _asbp_target_actor))

(event EventEnableTarget
  (params (Timeout :type Float%20%28double-precision%29) (Location :type Vector :default "0, 0, 0"))
  ;[1 1 1] Implemantaion Guide
  ;;[1 1 1] 3. Add This Functions inside BP
  (Default|DiscoverTarget (Variables|Default|GetBP%20Target%20Actor) Timeout (Variables|Default|GetCube) Location))

(fn ConstructionScript)